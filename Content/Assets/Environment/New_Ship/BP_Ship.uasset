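; BP_Ship is an environment ship Blueprint that animates the yaw of its lower sail component, ShipSailDown.
; On BeginPlay it picks a random negative start angle and a random positive end angle, so the swing can differ per instance.
; The TimelineSailDown track then drives a Lerp between those angles, setting the sail's relative rotation on each update.
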(event EventBeginPlay
  (Variables|Default|SetStartPoint (Math|Random|RandomFloatinRange -2e+01 -5e+01))
  (Variables|Default|SetEndPoint (Math|Random|RandomFloatinRange 2e+01 5e+01))
  (bind _newtrackrotationsaildown (Timeline|TimelineSailDown Play)
    (:Update
      (Transformation|SetRelativeRotation (Variables|Default|GetShip_SailDown) (Math|Rotator|MakeRotator 0.0 0.0 (Math|Float|Lerp (Variables|Default|GetStartPoint) (Variables|Default|GetEndPoint) _newtrackrotationsaildown)) false false))))

(fn ConstructionScript)